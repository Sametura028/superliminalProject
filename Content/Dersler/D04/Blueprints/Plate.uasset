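; Pressure plate actor that opens a Door while something overlaps its Box trigger.
; BeginPlay caches the door found by GetActorOfClass, so the plate has no per-instance door link.
; A single Timeline raises the door mesh and sinks the plate platform on overlap, then reverses when any overlap ends.
; Disconnected material-change nodes remain in the graph and never run.
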(event OnComponentBeginOverlap(Box)
  (params (OverlappedComponent :type Primitive%20Component%20Object%20Reference) (OtherActor :type Actor%20Object%20Reference) (OtherComp :type Primitive%20Component%20Object%20Reference) (OtherBodyIndex :type Integer) (bFromSweep :type Boolean) (SweepResult :type Hit%20Result%20Structure%20%28by%20ref%29))
  (Actor|GetActorOfClass 0)
  (bind _1 (Timeline|Timeline Play)
    (:Update
      (Transformation|SetRelativeLocation (Variables|/Game/Dersler/D04/Blueprints/Door.Door_C|GetSM_Door1 (Variables|Default|GetAs%20Door)) (Math|Vector|MakeVector 0.0 0.0 (* _1 2.5e+02)) false false)
      (Transformation|SetRelativeLocation (Variables|Default|GetSM_PressurePlate_Platform) (Math|Vector|MakeVector 0.0 0.0 (* _1 -1e+01)) false false))))

(event OnComponentEndOverlap(Box)
  (params (OverlappedComponent :type Primitive%20Component%20Object%20Reference) (OtherActor :type Actor%20Object%20Reference) (OtherComp :type Primitive%20Component%20Object%20Reference) (OtherBodyIndex :type Integer))
  (bind _1 (Timeline|Timeline Reverse)
    (:Update
      (Transformation|SetRelativeLocation (Variables|/Game/Dersler/D04/Blueprints/Door.Door_C|GetSM_Door1 (Variables|Default|GetAs%20Door)) (Math|Vector|MakeVector 0.0 0.0 (* _1 2.5e+02)) false false)
      (Transformation|SetRelativeLocation (Variables|Default|GetSM_PressurePlate_Platform) (Math|Vector|MakeVector 0.0 0.0 (* _1 -1e+01)) false false))))

(event EventBeginPlay
  (bind _returnvalue (Actor|GetActorOfClass "/Game/Dersler/D04/Blueprints/Door.Door_C"))
  (Variables|Default|SetAs%20Door _returnvalue))

(event Collision|EventActorBeginOverlap
  (params (OtherActor :type Actor%20Object%20Reference)))

(event EventTick
  (params (DeltaSeconds :type Float%20%28single-precision%29)))

(fn ConstructionScript)